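; Shooting-range target that awards points to the TrainMode game mode when AffectHealth fires.
; The construction script randomly picks a static, horizontal or vertical behavior and sets its score accordingly.
; On BeginPlay, a timeline lerps moving targets' Target component toward a random offset on the chosen axis.
; A hit adds score, stops movement, slides the component along Y through a looping timer, then destroys the actor after a short delay.
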(event Custom|MoveBack
  (bind _target (Variables|Default|GetTarget))
  ;[1 1 1] 受击得分
  (Transformation|SetRelativeLocation _target (+ (Variables|/Script/Engine.SceneComponent|GetRelativeLocation _target) "0,10.000000, 0") false false))

(event EventBeginPlay
  (bind _returnvalue (Math|Random|RandomFloatinRange 5e+01 1.5e+02))
  ;[1 1 1] 设置移动行为
  (switch Utilities|FlowControl|Switch|SwitchonTargetBehavior (Variables|Default|GetBehavior)
    (:NewEnumerator1
      (Variables|Default|SetDestinationLocation (Math|Vector|MakeVector _returnvalue 0.0 0.0))
      (bind _alpha (Timeline|T_Move PlayFromStart)
        (:Update
          (switch Utilities|FlowControl|Switch|SwitchonTargetBehavior (Variables|Default|GetBehavior)
            (:NewEnumerator1
              _)
            (:NewEnumerator2
              _))
          (Transformation|SetRelativeLocation (Variables|Default|GetTarget) (Math|Vector|Lerp(Vector) "0, 0, 0" (Variables|Default|GetDestinationLocation) _alpha) false false))))
    (:NewEnumerator2
      (Variables|Default|SetDestinationLocation (Math|Vector|MakeVector 0.0 0.0 _returnvalue))
      (Timeline|T_Move PlayFromStart))))

(event EventAffectHealth
  (params (delta :type Float%20%28single-precision%29))
  ;[1 1 1] 受击得分
  (bind _astrain_mode (Utilities|Casting|CastToTrainMode (Game|GetGameMode)))
  (Default|IncrementScore _astrain_mode (Variables|Default|GetScore))
  (Audio|Components|Audio|Stop (Variables|Default|GetT_Move))
  (Utilities|Time|SetTimerbyEvent (delegate Custom|MoveBack) 0.01 true)
  (Utilities|FlowControl|Delay 1.0)
  (Actor|DestroyActor))

(fn ConstructionScript
  (bind _output_get (Variables|Default|SetBehavior (Utilities|Enum|ByteToEnumTargetBehavior (Math|Conversions|ToByte(Integer) (Math|Random|RandomIntegerinRange 0 2)))))
  (switch Utilities|FlowControl|Switch|SwitchonTargetBehavior _output_get
    (:NewEnumerator0
      (Variables|Default|SetScore 50))
    (:NewEnumerator1
      (Variables|Default|SetScore 75))
    (:NewEnumerator2
      (Variables|Default|SetScore 100))))