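; Player-controlled shooter hero character that moves, jumps and drives an attached weapon.
; BeginPlay spawns the weapon on the gun socket, records its spawn transform in ShooterMode and creates two HUD widgets.
; Input forwards fire, rain fire and grenade actions to the weapon, and toggles its light and material.
; AffectHealth handles damage; death disables input, then after a delay requests respawn and destroys weapon and character.
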(event Custom|RainFire
  ;[1 1 1] 操作
  (Default|RainFire (Variables|Default|GetWeapon)))

(event Custom|FireGrenade
  ;[1 1 1] 操作
  (Default|FireGrenade (Variables|Default|GetWeapon)))

(event Custom|PullTrigger
  ;[1 1 1] 操作
  (Default|PullTrigge (Variables|Default|GetWeapon)))

(event Custom|RealeaseTrigger
  ;[1 1 1] 操作
  (Default|ReleaseTrigger (Variables|Default|GetWeapon)))

(event EventBeginPlay
  ;[1 1 1] 初始化
  (Utilities|FlowControl|Sequence
    (:then_0
      (CallFunction|SetupWeapon))
    (:then_1
      (CallFunction|SetupPlayerStart))
    (:then_2
      (CallFunction|SetupShooterHud))
    (:then_3
      (CallFunction|SetupInputHud))))

(event EventAffectHealth
  (params (delta :type Float%20%28single-precision%29))
  ;[1 1 1] 受伤接口
  (Class|BaseCharacter|CalculateHealth delta)
  (if (Variables|Default|GetisDead)
    (Input|DisableInput 0)
    (Default|ReleaseTrigger (Variables|Default|GetWeapon))
    (Utilities|FlowControl|Delay 3.0)
    (Default|RespawnPlayer (Variables|Default|GetGameMode))
    (Actor|DestroyActor (Variables|Default|GetWeapon))
    (Actor|DestroyActor)))

(event Input|ActionEvents|InputActionToggleWeaponLight
  (params (Key :type Key%20Structure :default "None"))
  ;[1 1 1] 操作
  (:Pressed
    (CallFunction|ToggleWeaponLight)))

(event Input|ActionEvents|InputActionJump
  (params (Key :type Key%20Structure :default "None"))
  ;[1 1 1] 输入
  ;;[1 1 1] 按键跳跃
  (:Pressed
    (Character|Jump))
  (:Released
    (Character|StopJumping)))

(event Input|ActionEvents|InputActionRainFire
  (params (Key :type Key%20Structure :default "None"))
  ;[1 1 1] 操作
  (:Pressed
    (CallFunction|RainFire)))

(event Input|ActionEvents|InputActionFireGrenade
  (params (Key :type Key%20Structure :default "None"))
  ;[1 1 1] 操作
  (:Pressed
    (CallFunction|FireGrenade)))

(event Input|ActionEvents|InputActionChangeWeaponMaterial
  (params (Key :type Key%20Structure :default "None"))
  ;[1 1 1] 操作
  (:Pressed
    (CallFunction|ChangeWeaponMaterial)))

(event Input|ActionEvents|InputActionshoot
  (params (Key :type Key%20Structure :default "None"))
  ;[1 1 1] 操作
  (:Pressed
    (CallFunction|PullTrigger))
  (:Released
    (CallFunction|RealeaseTrigger)))

(event Input|AxisEvents|InputAxisMoveRight
  (params (AxisValue :type Float%20%28single-precision%29))
  ;[1 1 1] 输入
  ;;[1 1 1] 移动操作
  (Pawn|Input|AddMovementInput (Math|Vector|GetRightVector (Math|Rotator|MakeRotator 0.0 0.0 (.Yaw (Math|Rotator|BreakRotator (Pawn|GetControlRotation :!class /Script/Engine.Pawn))))) AxisValue false))

(event Input|AxisEvents|InputAxisLookUp
  (params (AxisValue :type Float%20%28single-precision%29))
  ;[1 1 1] 输入
  ;;[1 1 1] 旋转视角
  (Pawn|Input|AddControllerPitchInput AxisValue))

(event Input|AxisEvents|InputAxisTurn
  (params (AxisValue :type Float%20%28single-precision%29))
  ;[1 1 1] 输入
  ;;[1 1 1] 旋转视角
  (Pawn|Input|AddControllerYawInput AxisValue))

(event Input|AxisEvents|InputAxisTurnRate
  (params (AxisValue :type Float%20%28single-precision%29))
  ;[1 1 1] 输入
  ;;[1 1 1] 旋转视角
  (Pawn|Input|AddControllerYawInput (* AxisValue (Variables|Default|GetBaseTurnRate) (Utilities|Time|GetWorldDeltaSeconds))))

(event Input|AxisEvents|InputAxisLookUpRate
  (params (AxisValue :type Float%20%28single-precision%29))
  ;[1 1 1] 输入
  ;;[1 1 1] 旋转视角
  (Pawn|Input|AddControllerPitchInput (* AxisValue (Variables|Default|GetBaseLookUpRate) (Utilities|Time|GetWorldDeltaSeconds))))

(event Input|AxisEvents|InputAxisMoveForward
  (params (AxisValue :type Float%20%28single-precision%29))
  ;[1 1 1] 输入
  ;;[1 1 1] 移动操作
  (Pawn|Input|AddMovementInput (Math|Vector|GetForwardVector (Math|Rotator|MakeRotator 0.0 0.0 (.Yaw (Math|Rotator|BreakRotator (Pawn|GetControlRotation :!class /Script/Engine.Pawn))))) AxisValue false))

(event Input|TouchEvents|InputTouch
  (params (Location :type Vector) (FingerIndex :type ETouchIndex%20Enum))
  ;[1 1 1] 输入
  ;;[1 1 1] 点击跳跃
  (:Pressed
    (Character|Jump))
  (:Released
    (Character|StopJumping)))

(fn ConstructionScript)

(fn CanFire
  (if (Variables|Default|GetisDead)
    _
    (elif (AI|Components|NavMovement|IsFalling (Variables|Character|GetCharacterMovement))
      _
      (else
        (bind _asthird_person_anim_bp (Utilities|Casting|CastToThirdPerson_AnimBP (Components|SkeletalMesh|GetAnimInstance (Variables|Character|GetMesh))))
        (return (<= (Variables|/Game/Mannequin/Animations/ThirdPerson_AnimBP.ThirdPerson_AnimBP_C|GetSpeed _asthird_person_anim_bp) 3e+02)))))
  (return false))

(fn ToggleHud
  (params (on :type Boolean))
  (bind _shooterhud (Variables|Default|GetShooterHud))
  (bind _inputhud (Variables|Default|GetInputHud))
  (if on
    (UserInterface|Viewport|AddtoViewport _shooterhud 0)
    (UserInterface|Viewport|AddtoViewport _inputhud 0)
    (else
      (Widget|RemovefromParent _shooterhud)
      (Widget|RemovefromParent _inputhud))))

(fn ToggleWeaponLight
  (bind _weapon (Variables|Default|GetWeapon))
  (bind _spotlight (Variables|/Game/game/blueprints/Weapon/Weapon.Weapon_C|GetSpotLight _weapon))
  (if (== (Variables|/Script/Engine.LightComponentBase|GetIntensity _spotlight) 0.0)
    (Rendering|Components|Light|SetIntensity _spotlight 5e+04)
    (else
      (Rendering|Components|Light|SetIntensity _spotlight 0.0))))

(fn ChangeWeaponMaterial
  (bind _weapon (Variables|Default|GetWeapon))
  (bind _gunmesh (Variables|/Game/game/blueprints/Weapon/Weapon.Weapon_C|GetGunMesh _weapon))
  (if (== (Rendering|Material|GetMaterial _gunmesh 0) "/Game/FPWeapon/Materials/MI_FPGun.MI_FPGun")
    (Rendering|Material|SetMaterial _gunmesh 0 "/Game/game/materials/M_Special.M_Special")
    (else
      (Rendering|Material|SetMaterial _gunmesh 0 "/Game/FPWeapon/Materials/MI_FPGun.MI_FPGun"))))

(fn SetupWeapon
  (bind _returnvalue (Game|SpawnActorfromClass "/Game/game/blueprints/Weapon/Weapon.Weapon_C" (Transformation|GetWorldTransform (Variables|Character|GetMesh)) "Undefined" 0 0))
  (bind _output_get (Variables|Default|SetWeapon _returnvalue))
  (Transformation|AttachComponentToComponent _output_get (Variables|Character|GetMesh) "GunSocket" "SnapToTarget" "KeepWorld" "KeepWorld" true))

(fn SetupPlayerStart
  (bind _asshooter_mode (Utilities|Casting|CastToShooterMode (Game|GetGameMode)))
  (bind _output_get (Variables|Default|SetGameMode _asshooter_mode))
  (Variables|/Game/game/blueprints/Mode/ShooterMode.ShooterMode_C|SetPlayerSpawnTransform _output_get (Transformation|GetActorTransform)))

(fn SetupShooterHud
  (bind _returnvalue (UserInterface|CreateWidget "/Game/game/widgets/ShooterHud.ShooterHud_C"))
  (bind _output_get (Variables|Default|SetShooterHud _returnvalue))
  (UserInterface|Viewport|AddtoViewport _output_get 0))

(fn SetupInputHud
  (bind _returnvalue (UserInterface|CreateWidget "/Game/game/widgets/InputHud.InputHud_C"))
  (bind _output_get (Variables|Default|SetInputHud _returnvalue))
  (UserInterface|Viewport|AddtoViewport _output_get 0))