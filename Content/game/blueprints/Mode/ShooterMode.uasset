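; ShooterMode is a shooter game mode that drives enemy spawning, player respawn and score keeping.
; On BeginPlay it finds the first EnemySpawner and sets a looping timer that calls its SpawnEnemy by name at the EnemySpawnPerSecond rate.
; RespawnPlayer destroys every enemy and its weapon, then spawns a new HeroCharacter at PlayerSpawnTransform for player controller 0 to possess.
; IncrementScore adds a given delta to Score.
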(event Custom|RespawnPlayer
  ;[1 1 1] 重新生成玩家
  (bind _outactors (Actor|GetAllActorsOfClass "/Game/game/blueprints/Character/EnemyCharacter.EnemyCharacter_C"))
  (for _array_element _outactors
    (Actor|DestroyActor (Variables|/Game/game/blueprints/Character/EnemyCharacter.EnemyCharacter_C|GetWeapon _array_element))
    (Actor|DestroyActor _array_element))
  (bind _returnvalue (Game|SpawnActorfromClass "/Game/game/blueprints/Character/HeroCharacter.HeroCharacter_C" (Variables|Default|GetPlayerSpawnTransform) "Undefined" 0 0))
  (Pawn|Possess (Game|GetPlayerController 0) _returnvalue))

(event Custom|IncrementScore
  (params (DeltaScore :type Integer))
  ;[1 1 1] 增加分数
  (Variables|Default|SetScore (+ DeltaScore (Variables|Default|GetScore))))

(event EventBeginPlay
  ;[1 1 1] 生成敌人
  (bind _outactors (Actor|GetAllActorsOfClass "/Game/game/blueprints/Spawner/EnemySpawner.EnemySpawner_C"))
  (bind _output_get (Variables|Default|SetSpawner (Utilities|Array|Get(acopy) _outactors)))
  (Utilities|Time|SetTimerbyFunctionName _output_get "SpawnEnemy" (/ 1.0 (Variables|Default|GetEnemySpawnPerSecond)) true))

(fn ConstructionScript)