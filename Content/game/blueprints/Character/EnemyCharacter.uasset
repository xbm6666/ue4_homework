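; Enemy character that carries a weapon, deals contact damage to the hero and awards score on death.
; BeginPlay attaches a spawned weapon to GunSocket, and the construction script tints the body through a dynamic material.
; Overlapping a HeroCharacter starts a looping damage timer at the attack rate, cleared on end overlap.
; AffectHealth updates health; on death it increments ShooterMode score, ignores WorldDynamic collision, detaches the controller, then destroys weapon and self after a delay.
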(event Custom|DamageTheHero
  ;[1 1 1] 靠近玩家时造成伤害
  (if (not (Variables|Default|GetisDead))
    (Default|AffectHealth (Variables|Default|GetHero) (Variables|Default|GetDamage))))

(event EventBeginPlay
  ;[1 1 1] 初始化：添加武器
  (bind _returnvalue (Game|SpawnActorfromClass "/Game/game/blueprints/Weapon/Weapon.Weapon_C" (Transformation|GetWorldTransform (Variables|Character|GetMesh)) "AdjustIfPossibleButAlwaysSpawn" 0 0))
  (bind _output_get (Variables|Default|SetWeapon _returnvalue))
  (Transformation|AttachComponentToComponent _output_get (Variables|Character|GetMesh) "GunSocket" "SnapToTarget" "KeepWorld" "KeepWorld" true))

(event Collision|EventActorBeginOverlap
  (params (OtherActor :type Actor%20Object%20Reference))
  ;[1 1 1] 靠近玩家时造成伤害
  (bind _ashero_character (Utilities|Casting|CastToHeroCharacter OtherActor))
  (Variables|Default|SetHero _ashero_character)
  (Utilities|Time|SetTimerbyFunctionName 0 "DamageTheHero" (/ 1.0 (Variables|Default|GetAttacksPerSecond)) true))

(event EventAffectHealth
  (params (delta :type Float%20%28single-precision%29))
  ;[1 1 1] 受伤接口
  (Class|BaseCharacter|CalculateHealth delta)
  (if (Variables|Default|GetisDead)
    (bind _asshooter_mode (Utilities|Casting|CastToShooterMode (Game|GetGameMode)))
    (Default|IncrementScore _asshooter_mode (Variables|Default|GetDelta%20Score))
    (Collision|SetCollisionResponsetoChannel (Variables|Default|GetCapsuleComponent) "ECC_WorldDynamic" "ECR_Ignore")
    (Class|Pawn|DetachfromControllerPendingDestroy)
    (Utilities|FlowControl|Delay 3.0)
    (Actor|DestroyActor (Variables|Default|GetWeapon))
    (Actor|DestroyActor)))

(event Collision|EventActorEndOverlap
  (params (OtherActor :type Actor%20Object%20Reference))
  ;[1 1 1] 靠近玩家时造成伤害
  (if (== OtherActor (Variables|Default|GetHero))
    (Utilities|Time|ClearTimerbyFunctionName 0 "DamageTheHero")))

(fn ConstructionScript
  (bind _returnvalue (Rendering|Material|CreateDynamicMaterialInstance (Variables|Character|GetMesh) 0 0 "None" :!class /Script/Engine.PrimitiveComponent))
  (bind _output_get (Variables|Default|SetdynaMat _returnvalue))
  (Rendering|Material|SetVectorParameterValue _output_get "BodyColor" (Variables|Default|GetenemyColor) :!class /Script/Engine.MaterialInstanceDynamic))