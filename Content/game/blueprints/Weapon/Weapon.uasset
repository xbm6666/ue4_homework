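; Weapon Blueprint that fires projectiles and grenades from a spawn point, with random fire sounds for gunshots.
; Trigger pull fires once behind a DoOnce, then repeats on a looping timer at RoundsPerSecond until release.
; RainFire spawns a 180-degree yaw fan of projectiles, and FireGrenade launches a Grenade.
; All shots check player 0's HeroCharacter CanFire, though normal Fire also shoots when that cast fails.
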(event Custom|PullTrigge
  ;[1 1 1] 按下与释放扳机
  (Utilities|FlowControl|DoOnce false
    (:Completed
      (CallFunction|Fire)
      (Utilities|Time|SetTimerbyFunctionName 0 "Fire" (/ 1.0 (Variables|Default|GetRoundsPerSecond)) true))))

(event Custom|ReleaseTrigger
  ;[1 1 1] 按下与释放扳机
  (Utilities|Time|ClearTimerbyFunctionName 0 "Fire")
  (Utilities|FlowControl|DoOnce false) ; enters at Reset
)

(event Custom|FireGrenade
  ;[1 1 1] 扔雷
  (bind _ashero_character (Utilities|Casting|CastToHeroCharacter (Game|GetPlayerCharacter 0)))
  (bind _canfire (Default|CanFire _ashero_character))
  (if _canfire
    (Game|SpawnActorfromClass "/Game/game/blueprints/Weapon/Grenade.Grenade_C" (Transformation|GetWorldTransform (Variables|Default|GetProjectieSpawnPoint)) "Undefined" 0 0)))

(event Custom|Fire
  ;[1 1 1] 实际射击行为
  (bind _ashero_character (Utilities|Casting|CastToHeroCharacter (Game|GetPlayerCharacter 0))
    (:then
      (bind _canfire (Default|CanFire _ashero_character))
      (if _canfire
        (Audio|PlaySoundatLocation (.OutItem (Utilities|Array|Random (Variables|Default|GetFireSounds))) (Transformation|GetWorldLocation (Variables|Default|GetGunMesh)) "0, 0, 0" 1.0 1.0 0.0 0 0 0 :!label _label)
        (Game|SpawnActorfromClass "/Game/game/blueprints/Weapon/projectile.projectile_C" (Transformation|GetWorldTransform (Variables|Default|GetProjectieSpawnPoint)) "Undefined" 0 0)))
    (:CastFailed
      (goto _label))))

(event Custom|RainFire
  (bind _projectiespawnpoint (Variables|Default|GetProjectieSpawnPoint))
  (bind _returnvalue (Transformation|GetWorldTransform _projectiespawnpoint))
  ;[1 1 1] 180度开火
  (bind _ashero_character (Utilities|Casting|CastToHeroCharacter (Game|GetPlayerCharacter 0)))
  (bind _canfire (Default|CanFire _ashero_character))
  (if _canfire
    (for _index (range 0 20)
      (Audio|PlaySoundatLocation (.OutItem (Utilities|Array|Random (Variables|Default|GetFireSounds))) (Transformation|GetWorldLocation (Variables|Default|GetGunMesh)) "0, 0, 0" 1.0 1.0 0.0 0 0 0)
      (Game|SpawnActorfromClass "/Game/game/blueprints/Weapon/projectile.projectile_C" (Math|Transform|MakeTransform (.location _returnvalue) (Math|Rotator|MakeRotator (.roll (.rotation _returnvalue)) (.pitch (.rotation _returnvalue)) (+ (.yaw (.rotation _returnvalue)) (- (* (Math|Conversions|ToFloat(Integer) _index) 9.0) 9e+01))) (.scale _returnvalue)) "Undefined" 0 0))))

(fn ConstructionScript)