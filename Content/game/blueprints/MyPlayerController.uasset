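; Player controller that toggles a pause menu from the pause input action.
; MyPause uses the PauseHud widget reference as the state: if valid it removes the menu and resumes, otherwise it creates the menu and pauses.
; Each toggle also switches the mouse cursor and calls ToggleHud on the HeroCharacter to hide or restore its HUD.
; Both branches set the input mode to Game and UI.
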(event Custom|MyPause
  ;[1 1 1] 暂停事件
  (Utilities|IsValid (Variables|Default|GetPauseHud)
    (:Is%20Valid
      (Widget|RemovefromParent (Variables|Default|GetPauseHud))
      (Variables|Default|SetPauseHud 0)
      (Input|SetInputModeGameandUI self 0 "DoNotLock" true)
      (Variables|Default|SetbShowMouseCursor false)
      (Game|SetGamePaused false)
      (bind _ashero_character (Utilities|Casting|CastToHeroCharacter (Game|GetPlayerCharacter 0)))
      (Default|ToggleHud _ashero_character true))
    (:Is%20Not%20Valid
      (bind _returnvalue (UserInterface|CreateWidget "/Game/game/widgets/PauseHud.PauseHud_C"))
      (bind _output_get (Variables|Default|SetPauseHud _returnvalue))
      (UserInterface|Viewport|AddtoViewport _output_get 0)
      (Input|SetInputModeGameandUI self 0 "DoNotLock" true)
      (Game|SetGamePaused true)
      (Variables|Default|SetbShowMouseCursor true)
      (bind _ashero_character_2 (Utilities|Casting|CastToHeroCharacter (Game|GetPlayerCharacter 0)))
      (Default|ToggleHud _ashero_character_2 false))))

(event EventBeginPlay)

(event EventTick
  (params (DeltaSeconds :type Float%20%28single-precision%29)))

(event Input|ActionEvents|InputActionpause
  (params (Key :type Key%20Structure :default "None"))
  ;[1 1 1] 暂停事件
  (:Pressed
    (CallFunction|MyPause)))

(fn ConstructionScript)