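; Enemy AI controller that runs the enemy behavior tree and feeds it what it perceives of the hero character.
; On BeginPlay it randomly sets a Blackboard flag for whether this enemy will flee at low HP.
; Perception updates write the sight and target keys on the Blackboard.
; Losing the hero clears sight immediately but clears the target after a short timer, which re-sensing cancels.
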(event OnTargetPerceptionUpdated(AIPerception)
  (params (Actor :type Actor%20Object%20Reference) (Stimulus :type AI%20Stimulus%20Structure))
  ;[1 1 1] 感知并设置玩家是否可见
  (bind _ashero_character (Utilities|Casting|CastToHeroCharacter Actor))
  (Variables|Default|SetPerceivedActor _ashero_character)
  (if (Utilities|Struct|BreakAIStimulus Stimulus)
    (CallFunction|UpdateSightKey true)
    (CallFunction|UpdateTargetKey (Variables|Default|GetPerceivedActor))
    (Utilities|Time|ClearandInvalidateTimerbyHandle (stale _returnvalue))
    (else
      (bind _returnvalue (Utilities|Time|SetTimerbyEvent (delegate Custom|LoseSight) 5.0))
      (CallFunction|UpdateSightKey false))))

(event Custom|LoseSight
  ;[1 1 1] 感知并设置玩家是否可见
  (CallFunction|UpdateTargetKey))

(event EventBeginPlay
  ;[1 1 1] 运行行为树并随机设置低血量是否逃跑
  (AI|RunBehaviorTree "/Game/game/blueprints/AI/EnemyBehaviorTree.EnemyBehaviorTree")
  (AI|Components|Blackboard|SetValueasBool (Variables|Default|GetBlackboard) (Variables|BehaviorTree|GetIsLowHPWillRun) (Math|Random|RandomBool)))

(fn ConstructionScript)

(fn UpdateSightKey
  (params (HasLineOfSight :type Boolean))
  (AI|Components|Blackboard|SetValueasBool (AI|GetBlackboard 0) (Variables|Default|GetSightKey) HasLineOfSight))

(fn UpdateTargetKey
  (params (TargetActor :type Actor%20Object%20Reference))
  (AI|Components|Blackboard|SetValueasObject (AI|GetBlackboard 0) (Utilities|Name|MakeLiteralName "TargetActor") TargetActor))