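; Spawner actor that populates a box area with Target actors for a timed round, started on BeginPlay.
; SpawnTargets destroys all existing Targets, spawns an initial batch, then runs a looping timer that adds one every second until a delay of about 15 seconds clears it.
; Each Target spawns at a random point inside the SpawnerArea bounds, ignoring collisions.
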(event Custom|SpawnTargets
  ;[1 1 1] 生成靶子
  (bind _outactors (Actor|GetAllActorsOfClass "/Game/game/blueprints/Target/Target.Target_C"))
  (for _array_element _outactors
    (Actor|DestroyActor _array_element))
  (for _index (range 0 5)
    (CallFunction|SpawnTarget))
  (bind _returnvalue (Utilities|Time|SetTimerbyEvent (delegate Custom|SpawnTarget) 1.0 true))
  (Utilities|FlowControl|Delay 15.5)
  (Utilities|Time|ClearandInvalidateTimerbyHandle _returnvalue))

(event Custom|SpawnTarget
  (bind _spawnerarea (Variables|Default|GetSpawnerArea))
  ;[1 1 1] 生成靶子
  (Game|SpawnActorfromClass "/Game/game/blueprints/Target/Target.Target_C" (Math|Transform|MakeTransform (Math|Random|RandomPointinBoundingBox (Transformation|GetWorldLocation _spawnerarea) (Components|Box|GetScaledBoxExtent _spawnerarea)) "0, 0, 0" "1,1,1") "AlwaysSpawn" 0 0))

(event EventBeginPlay
  ;[1 1 1] 生成靶子
  (CallFunction|SpawnTargets))

(fn ConstructionScript)