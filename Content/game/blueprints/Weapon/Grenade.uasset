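; Thrown grenade actor that explodes two seconds after spawning or on hitting an EnemyCharacter.
; BeginPlay launches the mesh forward and upward with an added force.
; Boom hides it, plays effects and gathers nearby EnemyCharacters with a sphere trace that ignores the player.
; A looping timer fakes knockback by nudging enemies away without sweep, then after a short delay they take damage and the grenade is destroyed.
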(event OnComponentHit(Grenade)
  (params (HitComponent :type Primitive%20Component%20Object%20Reference) (OtherActor :type Actor%20Object%20Reference) (OtherComp :type Primitive%20Component%20Object%20Reference) (NormalImpulse :type Vector :default "0, 0, 0") (Hit :type Hit%20Result%20Structure%20%28by%20ref%29))
  ;[1 1 1] 碰撞爆炸
  (if (Rendering|IsVisible (Variables|Default|GetGrenade))
    (Utilities|Casting|CastToEnemyCharacter OtherActor)
    (CallFunction|Boom)))

(event Custom|Boom
  (bind _grenade (Variables|Default|GetGrenade))
  (bind _returnvalue (Transformation|GetWorldLocation _grenade))
  ;[1 1 1] 爆炸事件
  (Rendering|SetVisibility (Variables|Default|GetGrenade) false false)
  (Audio|SpawnSoundatLocation "/Game/MobileStarterContent/Audio/Explosion01.Explosion01" _returnvalue "0, 0, 0" 0.7 1.0 0.0 0 0)
  (Effects|SpawnEmitteratLocation "/Game/MobileStarterContent/Particles/P_Explosion.P_Explosion" _returnvalue)
  (bind _outhits (Collision|MultiSphereTraceForObjects _returnvalue (+ _returnvalue "1.000000,1.000000,1.000000") 3e+02 (Variables|Default|GetObject%20Types) false (Utilities|Array|MakeArray (Game|GetPlayerCharacter 0)) "ForDuration"))
  (for _array_element _outhits
    (bind _asenemy_character (Utilities|Casting|CastToEnemyCharacter (.HitActor (Collision|BreakHitResult _array_element))))
    (Utilities|Array|Add (Variables|Default|GetEnemyCharacters) _asenemy_character))
  (bind _returnvalue_2 (Utilities|Time|SetTimerbyEvent (delegate Custom|MoveBack) 0.01 true))
  (Utilities|FlowControl|Delay 0.5)
  (Utilities|Time|ClearandInvalidateTimerbyHandle _returnvalue_2)
  (for _array_element_2 (Variables|Default|GetEnemyCharacters)
    (Default|AffectHealth _array_element_2 -5e+01))
  (Actor|DestroyActor))

(event Custom|MoveBack
  ;[1 1 1] 爆炸事件
  (for _array_element (Variables|Default|GetEnemyCharacters)
    (Transformation|SetActorLocation _array_element (+ (Transformation|GetActorLocation _array_element) (* (Math|Vector|Normalize (- (Transformation|GetActorLocation _array_element) (Transformation|GetWorldLocation (Variables|Default|GetGrenade)))) 5)) false false)))

(event EventBeginPlay
  (bind _grenade (Variables|Default|GetGrenade))
  ;[1 1 1] 添加初始推力并设置一定时间后爆炸
  (Transformation|SetWorldScale3D _grenade "0.250000,0.250000,0.250000")
  (Physics|AddForce _grenade (+ (* (Math|Rotator|GetRotationXVector (Transformation|GetWorldRotation _grenade)) "50000.000000,50000.000000,50000.000000") "0.000000,0.000000,30000.000000") "None" true)
  (Utilities|FlowControl|Delay 2.0)
  (CallFunction|Boom))

(fn ConstructionScript)