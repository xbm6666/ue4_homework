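; Weapon projectile Blueprint that deals damage to whatever damageable actor it overlaps.
; On overlap with an actor implementing IDamageable, it sends Damage through the AffectHealthMessage interface call.
; It then plays a random hit sound at its collision component and spawns a LaserSparks emitter at its transform.
; The projectile destroys itself on any overlap, with impact effects only for damageable targets.
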(event Collision|EventActorBeginOverlap
  (params (OtherActor :type Actor%20Object%20Reference))
  (bind _returnvalue (Transformation|GetActorTransform))
  (if (Utilities|DoesObjectImplementInterface OtherActor "/Game/game/blueprints/Weapon/iDamageable.iDamageable_C")
    (Class|IDamageable|AffectHealth(Message) OtherActor (Variables|Default|GetDamage))
    (Audio|PlaySoundatLocation (.OutItem (Utilities|Array|Random (Variables|Default|GetHitSounds))) (Transformation|GetWorldLocation (Variables|Default|GetProjectileCollision)) "0, 0, 0" 1.0 1.0 0.0 0 0 0)
    (Effects|SpawnEmitteratLocation "/Game/MobileStarterContent/Particles/LaserSparks.LaserSparks" (.location _returnvalue) (.rotation _returnvalue) (.scale _returnvalue))
    (Actor|DestroyActor)
    (else
      (Actor|DestroyActor))))

(fn ConstructionScript)